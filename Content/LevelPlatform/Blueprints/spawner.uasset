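; Side-scroller level actor named spawner that works as a triggered moving hazard, with no spawning logic.
; When the player character overlaps TriggerBox, a timeline lerps Box1 from its current relative location toward the actor's local origin.
; Overlapping Box1 deals fixed damage through the character's TakeDamage call.
; Both overlaps print debug strings, the second showing the damage call's result.
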(event OnComponentBeginOverlap(TriggerBox)
  (params (OverlappedComponent :type Primitive%20Component%20Object%20Reference) (OtherActor :type Actor%20Object%20Reference) (OtherComp :type Primitive%20Component%20Object%20Reference) (OtherBodyIndex :type Integer) (bFromSweep :type Boolean) (SweepResult :type Hit%20Result%20Structure%20%28by%20ref%29))
  (bind _box1 (Variables|Default|GetBox1))
  (Utilities|Casting|CastTo2DSideScrollerCharacter OtherActor)
  (Development|PrintString "Hello")
  (bind _newtrack_1 (Timeline|Timeline_1 Play)
    (:Update
      (Transformation|SetRelativeLocation _box1 (Math|Vector|Lerp(Vector) (Variables|/Script/Engine.SceneComponent|GetRelativeLocation _box1) "0.000000, 0,0.000000" _newtrack_1) false false))))

(event OnComponentBeginOverlap(Box1)
  (params (OverlappedComponent :type Primitive%20Component%20Object%20Reference) (OtherActor :type Actor%20Object%20Reference) (OtherComp :type Primitive%20Component%20Object%20Reference) (OtherBodyIndex :type Integer) (bFromSweep :type Boolean) (SweepResult :type Hit%20Result%20Structure%20%28by%20ref%29))
  (bind _as2dside_scroller_character (Utilities|Casting|CastTo2DSideScrollerCharacter OtherActor))
  (bind _newhp (Default|TakeDamage _as2dside_scroller_character 10))
  (Development|PrintString (Utilities|String|ToString(Integer) _newhp)))

(event EventBeginPlay)

(event EventTick
  (params (DeltaSeconds :type Float%20%28single-precision%29)))

(fn ConstructionScript)