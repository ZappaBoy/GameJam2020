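; Flower pickup actor for a 2D side-scroller that awards points to the player character.
; When the character overlaps the Sphere, it adds 150 times the character's FlowersMultiplier to its FlowerPoints, prints the new total and destroys itself.
; A separate Box overlap only prints a debug string when the character enters it.
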(event OnComponentBeginOverlap(Box)
  (params (OverlappedComponent :type Primitive%20Component%20Object%20Reference) (OtherActor :type Actor%20Object%20Reference) (OtherComp :type Primitive%20Component%20Object%20Reference) (OtherBodyIndex :type Integer) (bFromSweep :type Boolean) (SweepResult :type Hit%20Result%20Structure%20%28by%20ref%29))
  (Utilities|Casting|CastTo2DSideScrollerCharacter OtherActor)
  (Development|PrintString "cia dp"))

(event OnComponentBeginOverlap(Sphere)
  (params (OverlappedComponent :type Primitive%20Component%20Object%20Reference) (OtherActor :type Actor%20Object%20Reference) (OtherComp :type Primitive%20Component%20Object%20Reference) (OtherBodyIndex :type Integer) (bFromSweep :type Boolean) (SweepResult :type Hit%20Result%20Structure%20%28by%20ref%29))
  (bind _as2dside_scroller_character (Utilities|Casting|CastTo2DSideScrollerCharacter OtherActor))
  (bind _output_get (Variables|/Game/LevelPlatform/2DSideScrollerBP/2DSideScrollerCharacter.2DSideScrollerCharacter_C|SetflowerPoints _as2dside_scroller_character (+ (Variables|/Game/LevelPlatform/2DSideScrollerBP/2DSideScrollerCharacter.2DSideScrollerCharacter_C|GetflowerPoints _as2dside_scroller_character) (* (Variables|/Game/LevelPlatform/2DSideScrollerBP/2DSideScrollerCharacter.2DSideScrollerCharacter_C|GetflowersMultiplier _as2dside_scroller_character) 150))))
  (Development|PrintString (Utilities|String|ToString(Integer) _output_get))
  (Actor|DestroyActor))

(fn ConstructionScript)